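; BP_MapGenerator builds a square grid map out of BP_GridCell actors when play begins.
; Two nested five-step loops spawn each cell at the world origin, then offset it along X and Y by its loop indices.
; Spacing comes from twice each spawned cell's actor-bounds extent, so cell size sets the layout instead of a fixed value.
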(event `self.ReceiveBeginPlay`
  (for _index (range 5)
    (for _index_2 (range 5)
      (bind _returnvalue (`|SpawnActorFromClass` "/Game/TestLevel/Classes/BP_GridCell.BP_GridCell_C" (`KismetMathLibrary.MakeTransform` (0.0 0.0 0.0)) "Undefined" "OverrideRootScale" null null))
      (`self.K2_AddActorWorldOffset` _returnvalue (`KismetMathLibrary.MakeVector` (* (* (.x (`.BoxExtent` (`self.GetActorBounds` _returnvalue false false))) 2.0) _index) (* (* (.y (`.BoxExtent` (`self.GetActorBounds` _returnvalue false false))) 2.0) _index_2)) false false))))

(fn `UserConstructionScript`)